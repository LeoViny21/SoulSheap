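; Base actor for inventory item effects, representing an item in the world with a mesh and a pick-up prompt.
; GetItemData looks up the item's data table row through the row handle on its BCPItemData component.
; The construction script applies that row's static mesh and materials to ItemMesh.
; LookAt returns "Pick Up {Item}" text using the row's name, and the event graph holds no active logic.
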(fn `GetItemData`
  (returns (ItemData :type "/Game/Inventory/ItemData/S_Item_Info Structure"))
  (bind (_itemdata_datatable _itemdata_rowname) (break `DataTableRowHandle` (`/Game/Inventory/ItemData/BCP_ItemData.ItemData` (`self.BCP_ItemData`))))
  (bind _returnvalue (`|GetDataTableRow` _itemdata_datatable _itemdata_rowname)
    (:`then`
      (return _returnvalue))))

(fn `LookAt`
  (returns (Message :type Text))
  (return (`|FormatText` "Pick Up {Item}" (`.Name_23_E828489C49946EAF1AE06394A0913F1C` (break `/Game/Inventory/ItemData/S_Item_Info` (`self.GetItemData`))))))

(fn `SetItemMesh`
  (`StaticMeshComponent.SetStaticMesh` (`self.ItemMesh`) (`.StaicMesh_10_227604274F6C5548B2E428AF809FB2CB` (break `/Game/Inventory/ItemData/S_Item_Mesh_Info` (`.Mesh_26_18527B364742BDE7C08D75AB4C46AA4F` (break `/Game/Inventory/ItemData/S_Item_Info` (`self.GetItemData`)))))))

(fn `SetMaterail`
  (for (_array_element _array_index) (`.Materails_13_D8B554E64474A1940E73C7AA217F903D` (break `/Game/Inventory/ItemData/S_Item_Mesh_Info` (`.Mesh_26_18527B364742BDE7C08D75AB4C46AA4F` (break `/Game/Inventory/ItemData/S_Item_Info` (`self.GetItemData`)))))
    (`PrimitiveComponent.SetMaterial` (`self.ItemMesh`) _array_index _array_element)))

(fn `UserConstructionScript`
  (`self.SetItemMesh`)
  (`self.SetMaterail`))