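; Animal spawner that, on BeginPlay, spawns AnimalAmout BP_Animal actors at random child points of its Arrows component.
; A random stream, fixed by Seed or reset when Seed is -1, picks each location and animal type from ArrayAnimals.
; Spawn points are re-appended every iteration, so locations can repeat, and AnimalCount records a separate random pick from the spawned type.
; A BP_Spawns path is disconnected; interface-style functions are stubs.
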(event `self.ReceiveBeginPlay`
  (`self.SetSeed`)
  (`self.SpawnAnimal`))

(fn `ENum`
  (returns (Out4 :type "/Game/Animals/E_Animal Enum"))
  (return "NewEnumerator0"))

(fn `GetSpawnPoints`
  (returns (SpawnPoints :type "Array of SceneComponent Object Reference"))
  (return))

(fn `IsInteracble`
  (returns (Stream :type "RandomStream Structure"))
  (return))

(fn `SetSeed`
  (bind _stream (`self.Stream`))
  (if (== (`self.Seed`) -1)
    (`KismetMathLibrary.ResetRandomStream` _stream)
    (else
      (`KismetMathLibrary.SetRandomStreamSeed` _stream (`self.Seed`)))))

(fn `SpawnAnimal`
  (locals (Spawn :type "Array of SceneComponent Object Reference") (Enum :type "/Game/Animals/E_Animal Enum" :default "NewEnumerator0") (EnumArray :type "Array of /Game/Animals/E_Animal Enum") (SelectedSpawn :type "SceneComponent Object Reference") (Animals :type "Array of /Game/Animals/E_Animal Enum") (RandomInt :type Integer) (SecondRandInt :type Integer) (ExitSpawns :type "Array of SceneComponent Object Reference"))
  (bind _spawn (`local.Spawn`))
  (bind _outitem (`KismetArrayLibrary.Array_RandomFromStream` (`self.ArrayAnimals`) (`self.Stream`)))
  (bind (_returnvalue_x _returnvalue_y _returnvalue_z) (`KismetMathLibrary.BreakVector` (`SceneComponent.K2_GetComponentLocation` (`local.SelectedSpawn`))))
  (bind _output_get (set `local.ExitSpawns` (`SceneComponent.GetChildrenComponents` (`self.Arrows`) false)))
  (for _ (range 1 (+ (`self.AnimalAmout`) 1))
    (`KismetArrayLibrary.Array_Append` _spawn _output_get)
    (set `local.SelectedSpawn` (`KismetArrayLibrary.Array_RandomFromStream` _spawn (`self.Stream`)))
    (`|SpawnActorFromClass` "/Game/Animals/BP_Animal.BP_Animal_C" (`KismetMathLibrary.MakeTransform` (`KismetMathLibrary.MakeVector` _returnvalue_x _returnvalue_y _returnvalue_z)) "AlwaysSpawn" "MultiplyWithRoot" null _outitem null)
    (`KismetArrayLibrary.Array_Add` (`self.AnimalCount`) _outitem)
    (`KismetArrayLibrary.Array_RemoveItem` (`local.Spawn`) (`local.SelectedSpawn`))))

(fn `UserConstructionScript`)