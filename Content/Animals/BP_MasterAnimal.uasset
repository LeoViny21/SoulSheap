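; BP_MasterAnimal is an animal Blueprint with unfinished logic for wandering and for selecting another animal for possession.
; BeginPlay calls RandMoveFun, which queries a random navigable point, discards it and recurses endlessly without moving.
; Sphere overlaps collect actors and pick one at random.
; A looping dungeon-check timer, not started here, runs PossessionCheck and re-arms itself; that check only re-picks and flags Possession if the pick is a BP_MasterAnimal.
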(event `self.ReceiveBeginPlay`
  (`self.RandMoveFun`))

(event `self.Sphere.OnComponentBeginOverlap`
  (params (OverlappedComponent :type "PrimitiveComponent Object Reference") (OtherActor :type "Actor Object Reference") (OtherComp :type "PrimitiveComponent Object Reference") (OtherBodyIndex :type Integer) (bFromSweep :type Boolean) (SweepResult :type "HitResult Structure (by ref)"))
  (`KismetArrayLibrary.Array_AddUnique` (`self.ActorArray`) OtherActor)
  (set `self.SelectAniaml` (`KismetArrayLibrary.Array_Random` (`self.ActorArray`))))

(event `self.Sphere.OnComponentEndOverlap`
  (params (OverlappedComponent :type "PrimitiveComponent Object Reference") (OtherActor :type "Actor Object Reference") (OtherComp :type "PrimitiveComponent Object Reference") (OtherBodyIndex :type Integer)))

(event `Start Dugeon TImer`
  (bind _returnvalue (`KismetSystemLibrary.K2_SetTimerDelegate` (delegate `Check For Dungen Complete`) 2.0 true))
  (set `self.TimerHandel` _returnvalue))

(event `Check For Dungen Complete`
  (`self.PossessionCheck`)
  (`self.Start Dugeon TImer`))

(fn `PossessionCheck`
  (if (not (`self.Possession`))
    (bind _output_get (set `self.SelectAniaml` (`KismetArrayLibrary.Array_Random` (`self.ActorArray`))))
    (cast `/Game/Animals/BP_MasterAnimal` _output_get)
    (set `self.Possession` true)))

(fn `RandMoveFun`
  (`NavigationSystemV1.K2_GetRandomLocationInNavigableRadius` (`self.K2_GetActorLocation`) 2000.0 null null)
  (`self.RandMoveFun` self))

(fn `SetAffection`)

(fn `UserConstructionScript`)