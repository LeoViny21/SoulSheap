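; BP_AnimalSpawner spawns animals at random floor spawn points of a farm actor when play begins.
; It seeds a random stream from Seed, or randomly when Seed is -1, to pick points.
; SpawnAnimal recursively spawns a farm, appends its points, then spawns a BP_Animal.
; Recursion stops only at zero AnimalAmout, which is never decremented; a selected animal overwrites Seed instead.
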(event `self.ReceiveBeginPlay`
  (`self.SetSeed`)
  (`self.SpawnAnimal`))

(fn `IsInteracble`
  (returns (Stream :type "RandomStream Structure"))
  (return))

(fn `SetSeed`
  (bind _stream (`self.Stream`))
  (if (== (`self.Seed`) -1)
    (`KismetMathLibrary.SeedRandomStream` _stream)
    (else
      (`KismetMathLibrary.SetRandomStreamSeed` _stream (`self.Seed`)))))

(fn `SpawnAnimal`
  (locals (Spawn :type "Array of SceneComponent Object Reference"))
  (bind _spawn (`local.Spawn`))
  (if (== (`self.AnimalAmout`) 0)
    (return)
    (else
      (bind _returnvalue (`|SpawnActorFromClass` "/Game/Platfrom/Base/BP_Farm.BP_Farm_C" (`SceneComponent.K2_GetComponentToWorld` (`self.DefaultSceneRoot`)) "AlwaysSpawn" "MultiplyWithRoot" null null))
      (`KismetArrayLibrary.Array_Append` _spawn (`SceneComponent.GetChildrenComponents` (`/Game/Platfrom/Base/BP_Farm.FloorSpawnPoints` _returnvalue) false))
      (bind _returnvalue_2 (`|SpawnActorFromClass` "/Game/Animals/BP_Animal.BP_Animal_C" (`KismetMathLibrary.Conv_VectorToTransform` (`SceneComponent.K2_GetComponentLocation` (`KismetArrayLibrary.Array_RandomFromStream` _spawn (`self.Stream`)))) "AlwaysSpawn" "MultiplyWithRoot" null null))
      (if (== (`/Game/Animals/BP_Animal.Selected` _returnvalue_2) 1)
        (set `self.Seed` (- (`self.AnimalAmout`) 1))
        (`self.SpawnAnimal`)
        (else
          (`self.SpawnAnimal`))))))

(fn `UserConstructionScript`)