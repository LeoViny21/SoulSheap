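; BP_Animal is a wandering animal that takes a sheep, bat, pro sheep or pro bat mesh in its construction script.
; From BeginPlay, CheckForPlayer loops AI moves to random navigable points, briefly spawning a pointer actor at each; despite its name, it detects no player.
; A sphere hit sets Pro, but only the construction script reads that flag.
; AnimalChance, Possession, ENum and IsInteracble are stubs.
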(event `self.ReceiveBeginPlay`
  (`self.CheckForPlayer`))

(event `CheckForPlayer`
  ; Check For Player
  (bind _randomlocation (`NavigationSystemV1.K2_GetRandomLocationInNavigableRadius` (`self.K2_GetActorLocation`) 1000.0 null null))
  (bind _returnvalue (`|SpawnActorFromClass` "/Game/Animals/BP_pointer.BP_pointer_C" (`KismetMathLibrary.Conv_VectorToTransform` _randomlocation) "Undefined" "MultiplyWithRoot" null null))
  (`KismetSystemLibrary.Delay` 0.2)
  (`self.K2_DestroyActor` _returnvalue)
  (`|AIMoveTo` self _randomlocation null 200.0
    (:`OnSuccess`
      _)
    (:`OnFail`
      _))
  (`self.CheckForPlayer`))

(event `self.Sphere.OnComponentHit`
  (params (HitComponent :type "PrimitiveComponent Object Reference") (OtherActor :type "Actor Object Reference") (OtherComp :type "PrimitiveComponent Object Reference") (NormalImpulse :type "Vector Structure") (Hit :type "HitResult Structure (by ref)"))
  (set `self.Pro` true)
  (`KismetSystemLibrary.Delay` 5.0))

(fn `AnimalChance`)

(fn `ENum`
  (returns (Out4 :type "/Game/Animals/E_Animal Enum"))
  (return "NewEnumerator0"))

(fn `IsInteracble`
  (returns (Stream :type "RandomStream Structure"))
  (return))

(fn `Possession`)

(fn `UserConstructionScript`
  (locals (Selection :type "/Game/Animals/E_Animal Enum" :default "NewEnumerator0"))
  (bind _mesh (`self.Mesh`))
  (bind _mesh_2 (`self.Mesh`))
  (switch `/Game/Animals/E_Animal` (`self.Selection_0`)
    (:`NewEnumerator0`
      (`SkeletalMeshComponent.SetSkeletalMeshAsset` _mesh "/Game/Animals/Meshes/Sheep/SheepJoinedCenter.SheepJoinedCenter")
      (if (`self.Pro`)
        (`SkeletalMeshComponent.SetSkeletalMeshAsset` _mesh_2 "/Game/Animals/Meshes/Sheep/ProSheepJoinedCenter.ProSheepJoinedCenter")))
    (:`NewEnumerator2`
      (`SkeletalMeshComponent.SetSkeletalMeshAsset` _mesh "/Game/Animals/Meshes/Bat/BatSmall/BatSmall.BatSmall"))
    (:`NewEnumerator3`
      (`SkeletalMeshComponent.SetSkeletalMeshAsset` _mesh "/Game/Animals/Meshes/Sheep/ProSheepJoinedCenter.ProSheepJoinedCenter")
      (if (`self.Pro`)
        (`SkeletalMeshComponent.SetSkeletalMeshAsset` _mesh_2 "/Game/Animals/Meshes/Bat/BatSmall/ProBatSmall.ProBatSmall")))
    (:`NewEnumerator4`
      (`SkeletalMeshComponent.SetSkeletalMeshAsset` _mesh "/Game/Animals/Meshes/Bat/BatSmall/ProBatSmall.ProBatSmall"))))