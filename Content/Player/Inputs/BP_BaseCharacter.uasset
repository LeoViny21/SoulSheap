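; Player character with Enhanced Input look, movement and adjustable fly speed, which interacts with BP_Animal actors.
; Movement follows control rotation, and the speed input scales MaxFlySpeed.
; Tick line-traces from the camera toward its forward vector times a large distance, without adding the start location, and calls ProSwitch on a hit BP_Animal.
; IA_Cure triggers the same ProSwitch call directly, while ReturnPro is a stub returning false.
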(event `EnhancedInput|/Game/Player/Inputs/IA_Look`
  (params (ActionValue :type "Vector2D Structure") (ElapsedSeconds :type "Float (double-precision)") (TriggeredSeconds :type "Float (double-precision)") (InputAction :type "InputAction Object Reference" :default "/Game/Player/Inputs/IA_Look.IA_Look"))
  (:`Triggered`
    (`self.AddControllerYawInput` ActionValue_X)
    (`self.AddControllerPitchInput` ActionValue_Y)))

(event `EnhancedInput|/Game/Player/Inputs/IA_MoveForward`
  (params (ActionValue :type "Float (double-precision)") (ElapsedSeconds :type "Float (double-precision)") (TriggeredSeconds :type "Float (double-precision)") (InputAction :type "InputAction Object Reference" :default "/Game/Player/Inputs/IA_MoveForward.IA_MoveForward"))
  (bind (_returnvalue_roll _returnvalue_pitch _returnvalue_yaw) (`KismetMathLibrary.BreakRotator` (`self.GetControlRotation`)))
  (:`Triggered`
    (`self.AddMovementInput` (`KismetMathLibrary.GetForwardVector` (`KismetMathLibrary.MakeRotator` _returnvalue_roll _returnvalue_pitch _returnvalue_yaw)) ActionValue)))

(event `EnhancedInput|/Game/Player/Inputs/IA_MoveRight`
  (params (ActionValue :type "Float (double-precision)") (ElapsedSeconds :type "Float (double-precision)") (TriggeredSeconds :type "Float (double-precision)") (InputAction :type "InputAction Object Reference" :default "/Game/Player/Inputs/IA_MoveRight.IA_MoveRight"))
  (bind (_returnvalue_roll _returnvalue_pitch _returnvalue_yaw) (`KismetMathLibrary.BreakRotator` (`self.GetControlRotation`)))
  (:`Triggered`
    (`self.AddMovementInput` (`KismetMathLibrary.GetRightVector` (`KismetMathLibrary.MakeRotator` _returnvalue_roll _returnvalue_pitch _returnvalue_yaw)) ActionValue)))

(event `EnhancedInput|/Game/Player/Inputs/IA_FlyingSpeed`
  (params (ActionValue :type "Float (double-precision)") (ElapsedSeconds :type "Float (double-precision)") (TriggeredSeconds :type "Float (double-precision)") (InputAction :type "InputAction Object Reference" :default "/Game/Player/Inputs/IA_FlyingSpeed.IA_FlyingSpeed"))
  (:`Triggered`
    (set `CharacterMovementComponent.MaxFlySpeed` (* ActionValue (`self.Max Fly Speed`)) (`self.CharacterMovement`))))

(event `self.ReceiveTick`
  (params (DeltaSeconds :type "Float (single-precision)"))
  (bind _camera (`self.Camera`))
  (bind _outhit (`KismetSystemLibrary.LineTraceSingle` :`Start` (`SceneComponent.K2_GetComponentLocation` _camera) :`End` (* (`KismetMathLibrary.GetForwardVector` (`SceneComponent.K2_GetComponentRotation` _camera)) 100000.0) :`TraceChannel` "TraceTypeQuery1" :`DrawDebugType` "ForDuration"))
  (bind (_bblockinghit _binitialoverlap _time _distance _location _impactpoint _normal _impactnormal _physmat _hitactor) (`GameplayStatics.BreakHitResult` _outhit))
  (if (== (`GameplayStatics.GetObjectClass` _hitactor) "/Game/Animals/BP_Animal.BP_Animal_C")
    (bind _asbp_animal (cast `/Game/Animals/BP_Animal` _hitactor)
      (:`then`
        (`/Game/Animals/BP_Animal.ProSwitch` _asbp_animal :!label _label))
      (:`CastFailed`
        (`KismetSystemLibrary.PrintString` "Fail")))))

(event `EnhancedInput|/Game/Player/Inputs/IA_Cure`
  (params (ActionValue :type Boolean) (ElapsedSeconds :type "Float (double-precision)") (TriggeredSeconds :type "Float (double-precision)") (InputAction :type "InputAction Object Reference" :default "/Game/Player/Inputs/IA_Cure.IA_Cure"))
  (:`Triggered`
    (goto _label)))

(fn `ReturnPro`
  (returns (Pro :type Boolean))
  (return false))

(fn `UserConstructionScript`)